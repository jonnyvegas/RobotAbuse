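; Player controller Blueprint that handles input setup, releasing a held BP_RARobot and quitting the game.
; After begin play it locks the mouse in game-and-UI mode, caches the robot and adds the IMC_RADefault mapping context.
; A raw left-mouse release clears the robot's held flag and restores look input, while Escape quits.
; The IA_ReleaseLMB action only prints debug text, and windowed-resolution setup is left unconnected.
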(event Input|EnhancedActionEvents|EnhancedInputActionIA_ReleaseLMB
  (params (ActionValue :type Boolean) (ElapsedSeconds :type Float%20%28double-precision%29) (TriggeredSeconds :type Float%20%28double-precision%29) (InputAction :type Input%20Action%20Object%20Reference :default "/Game/Blueprints/InputActions/Actions/IA_ReleaseLMB.IA_ReleaseLMB"))
  (:Started
    (Development|PrintString "lmb start"))
  (:Completed
    (Development|PrintString "lmb done")))

(event EventBeginPlay)

(event EventTick
  (params (DeltaSeconds :type Float%20%28single-precision%29)))

(event EventBPBeginPlayPost
  (Input|SetInputModeGameandUI self 0 "LockAlways" false false)
  (bind _returnvalue (Actor|GetActorOfClass "/Game/Blueprints/Robot/BP_RARobot.BP_RARobot_C"))
  (Variables|Default|SetRobotRef _returnvalue)
  (Input|AddMappingContext (PlayerController|LocalPlayerSubsystems|GetEnhancedInputLocalPlayerSubsystem) "/Game/Blueprints/InputActions/IMC_RADefault.IMC_RADefault" 0 "(bIgnoreAllPressedKeysUntilRelease=True,bForceImmediately=False,bNotifyUserSettings=False)"))

(event Input|MouseEvents|LeftMouseButton
  (params (Key :type Key%20Structure :default "None"))
  (bind _robotref (Variables|Default|GetRobotRef))
  (:Released
    (if (Variables|/Game/Blueprints/Robot/BP_RARobot.BP_RARobot_C|GetIsBeingHeld _robotref)
      (Variables|/Game/Blueprints/Robot/BP_RARobot.BP_RARobot_C|SetIsBeingHeld _robotref false)
      (Input|SetIgnoreLookInput false))))

(event Input|KeyboardEvents|Escape
  (params (Key :type Key%20Structure :default "None"))
  (:Pressed
    (Game|QuitGame 0 "Quit" false)))

(fn ConstructionScript)